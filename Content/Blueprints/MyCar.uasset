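; MyCar is a player-controlled car for an infinite runner that moves steadily along X and switches between three lanes.
; BeginPlay adds the CarController Enhanced Input mapping context, and Tick advances the car by a fixed, frame-rate-dependent step.
; Left and right input actions call ChangeLanes, which clamps the target index and lerps Y to that lane's position with the Transition timeline, updating the current lane when it finishes.
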(event Custom|Change%20Lanes
  (params (Shift%20Lanes :type Integer))
  (bind _returnvalue (Transformation|GetActorLocation))
  (bind (_x _y _z) (Math|Vector|BreakVector _returnvalue))
  ;[0.15 0.15 0.15 0.5] Change Lanes
  (Variables|Default|SetTargetLaneIndex (Math|Integer|Clamp(Integer) (+ Shift%20Lanes (Variables|Default|GetCurrentLane)) 0 2))
  (bind _output_get (Variables|Default|SetCurrentY (.Y (Math|Vector|BreakVector (Transformation|GetActorLocation)))))
  (bind _change_lanes (Timeline|Transition PlayFromStart)
    (:Update
      (Transformation|SetActorLocation (Math|Vector|MakeVector _x (Math|Float|Lerp _output_get (Utilities|Array|Get(acopy) (Variables|Default|GetLane%20Position) (Variables|Default|GetTargetLaneIndex)) _change_lanes) _z) false false))
    (:Finished
      (Variables|Default|SetCurrentLane (Variables|Default|GetTargetLaneIndex)))))

(event Input|EnhancedActionEvents|EnhancedInputActionLeft_IA
  (params (ActionValue :type Vector%202D%20Structure) (ElapsedSeconds :type Float%20%28double-precision%29) (TriggeredSeconds :type Float%20%28double-precision%29) (InputAction :type Input%20Action%20Object%20Reference :default "/Game/Blueprints/Left_IA.Left_IA"))
  ;[0.15 0.15 0.15 0.5] Change Lanes
  (CallFunction|ChangeLanes -1))

(event Input|EnhancedActionEvents|EnhancedInputActionRight_IA
  (params (ActionValue :type Boolean) (ElapsedSeconds :type Float%20%28double-precision%29) (TriggeredSeconds :type Float%20%28double-precision%29) (InputAction :type Input%20Action%20Object%20Reference :default "/Game/Blueprints/Right_IA.Right_IA"))
  ;[0.15 0.15 0.15 0.5] Change Lanes
  (CallFunction|ChangeLanes 1))

(event EventBeginPlay
  ;[0.15 0.15 0.15 0.5] Added Input Mapping
  (bind _asplayer_controller (Utilities|Casting|CastToPlayerController (Pawn|GetController)))
  (Utilities|IsValid (PlayerController|LocalPlayerSubsystems|GetEnhancedInputLocalPlayerSubsystem _asplayer_controller)
    (:Is%20Valid
      (Input|AddMappingContext (PlayerController|LocalPlayerSubsystems|GetEnhancedInputLocalPlayerSubsystem _asplayer_controller) "/Game/Blueprints/CarController.CarController" 0 "(bIgnoreAllPressedKeysUntilRelease=True,bForceImmediately=False,bNotifyUserSettings=False)"))))

(event EventTick
  (params (DeltaSeconds :type Float%20%28single-precision%29))
  (bind _returnvalue (Transformation|GetActorLocation))
  (bind (_x _y _z) (Math|Vector|BreakVector _returnvalue))
  ;[0.15 0.15 0.15 0.5] Infinite Run
  (Transformation|SetActorLocation (Math|Vector|MakeVector (+ _x 1e+01) _y _z) false false))

(fn ConstructionScript)